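; Base enemy Blueprint that shows a floating button prompt near the player and spawns BP_DeadEnnemi when destroyed.
; Sphere overlap reveals the widget if the player character is in a specific state.
; Timelines, with play rates set in the construction script, scale it and bob it above the capsule via FlipFlop until hovering ends.
; EffectUnderFeet is an empty stub and Grabbing just returns false.
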(event `self.ReceiveDestroyed`
  ;[0.8314 0.3255 0.3339] Destroyed
  (`|SpawnActorFromClass` "/Game/Gameplay/Enemies/BP_DeadEnnemi.BP_DeadEnnemi_C" (`self.GetTransform`) "Undefined" "OverrideRootScale" null null))

(event `self.ReceiveBeginPlay`
  (`SceneComponent.SetVisibility` (`self.HoverButtonWidget`) false true))

(event `self.ReceiveTick`
  (params (DeltaSeconds :type "Float (single-precision)")))

(event `self.CollisionSphere.OnComponentBeginOverlap`
  (params (OverlappedComponent :type "PrimitiveComponent Object Reference") (OtherActor :type "Actor Object Reference") (OtherComp :type "PrimitiveComponent Object Reference") (OtherBodyIndex :type Integer) (bFromSweep :type Boolean) (SweepResult :type "HitResult Structure (by ref)"))
  (if (== OtherActor (`GameplayStatics.GetPlayerCharacter` 0))
    (bind _output (`self.IsSelectedPlayerState` "NewEnumerator0"))
    (if _output
      (`self.HoverButtonStart`)
      (`self.EffectUnderFeet`))))

(event `self.CollisionSphere.OnComponentEndOverlap`
  (params (OverlappedComponent :type "PrimitiveComponent Object Reference") (OtherActor :type "Actor Object Reference") (OtherComp :type "PrimitiveComponent Object Reference") (OtherBodyIndex :type Integer))
  (if (== OtherActor (`GameplayStatics.GetPlayerCharacter` 0))
    (`self.HoverButtonEnd`)))

(event `EffectUnderFeet`)

(event `HoverButtonStart`
  (set `self.bHovering` true)
  (`SceneComponent.SetVisibility` (`self.HoverButtonWidget`) true false)
  (`self.HoverButtonToEndPos`)
  (bind (_direction _curve_scalebuttonhover_float) (`Timeline|HoveringButtonScaleTimeline` :!via `PlayFromStart`)
    (:`Update`
      (bind _returnvalue (`KismetMathLibrary.Lerp` 1.0 (`self.SizeHB`) _curve_scalebuttonhover_float))
      (`WidgetComponent.SetDrawSize` (`self.HoverButtonWidget`) (`KismetMathLibrary.MakeVector2D` _returnvalue _returnvalue)))))

(event `HoverButtonEnd`
  (set `self.bHovering` false)
  (bind (_direction _curve_scalebuttonhover_float) (`Timeline|HoveringButtonDownScaleTimeline` :!via `ReverseFromEnd`)
    (:`Update`
      (bind _returnvalue (`KismetMathLibrary.Lerp` 1.0 (`self.SizeHB`) _curve_scalebuttonhover_float))
      (`WidgetComponent.SetDrawSize` (`self.HoverButtonWidget`) (`KismetMathLibrary.MakeVector2D` _returnvalue _returnvalue)))
    (:`Finished`
      (`SceneComponent.SetVisibility` (`self.HoverButtonWidget`) true false))))

(event `HoverButtonToEndPos`
  (bind _hoverbuttonwidget (`self.HoverButtonWidget`))
  (bind (_returnvalue_x _returnvalue_y) (`KismetMathLibrary.BreakVector` (`SceneComponent.K2_GetComponentLocation` _hoverbuttonwidget)))
  (bind (_returnvalue_x_2 _returnvalue_y_2 _returnvalue_z) (`KismetMathLibrary.BreakVector` (`SceneComponent.K2_GetComponentLocation` (`self.CapsuleComponent`))))
  (bind _returnvalue (+ _returnvalue_z (`self.VerticalWorldOffsetHB`)))
  ;[0.3255 0.4588 0.8314] Hovering Loop
  (bind (_direction _curve_buttonhover_float) (`Timeline|HoverButtonTimeline` :!via `PlayFromStart` :!label _label)
    (:`Update`
      (`SceneComponent.K2_SetWorldLocation` _hoverbuttonwidget (`KismetMathLibrary.MakeVector` _returnvalue_x _returnvalue_y (`KismetMathLibrary.Lerp` _returnvalue (+ _returnvalue (`self.AmplitudeHB`)) _curve_buttonhover_float)) false false))
    (:`Finished`
      (if (`self.bHovering`)
        (`/Engine/EditorBlueprintResources/StandardMacros.FlipFlop`
          (:`A`
            (`self.HoverButtonToStartPos`))
          (:`B`
            (`self.HoverButtonToEndPos`)))
        (else
          (`self.ResetHoverButtonLocation`))))))

(event `HoverButtonToStartPos`
  ;[0.3255 0.4588 0.8314] Hovering Loop
  (goto _label :!via `ReverseFromEnd`))

(fn `Grabbing`
  (params (WhoGrabbed :type "Actor Object Reference"))
  (returns (CanBeGrabbed :type Boolean))
  (return false))

(fn `IsSelectedPlayerState`
  (params (DesiredState :type "/Game/Gameplay/Character/Character_States Enum" :default "NewEnumerator0"))
  (returns (Output :type Boolean))
  (bind _asbp_third_person_character (cast `/Game/Gameplay/BP_ThirdPersonCharacter` (`GameplayStatics.GetPlayerCharacter` 0)))
  (return (`|EnumEquality` (`/Game/Gameplay/BP_ThirdPersonCharacter.State` _asbp_third_person_character) DesiredState)))

(fn `ResetHoverButtonLocation`
  (bind _hoverbuttonwidget (`self.HoverButtonWidget`))
  (bind (_returnvalue_x _returnvalue_y) (`KismetMathLibrary.BreakVector` (`SceneComponent.K2_GetComponentLocation` _hoverbuttonwidget)))
  (bind (_returnvalue_x_2 _returnvalue_y_2 _returnvalue_z) (`KismetMathLibrary.BreakVector` (`SceneComponent.K2_GetComponentLocation` (`self.CapsuleComponent`))))
  (`SceneComponent.K2_SetWorldLocation` _hoverbuttonwidget (`KismetMathLibrary.MakeVector` _returnvalue_x _returnvalue_y (+ _returnvalue_z (`self.VerticalWorldOffsetHB`))) false false))

(fn `UserConstructionScript`
  (bind (_returnvalue_x _returnvalue_y _returnvalue_z) (`KismetMathLibrary.BreakVector` (`SceneComponent.K2_GetComponentLocation` (`self.HoverButtonWidget`))))
  (bind (_returnvalue_x_2 _returnvalue_y_2 _returnvalue_z_2) (`KismetMathLibrary.BreakVector` (`SceneComponent.K2_GetComponentLocation` (`self.CapsuleComponent`))))
  ;[0.5176 0.8314 0.3255] Hover Button
  (`SceneComponent.K2_AddLocalOffset` (`self.HoverButtonWidget`) (`KismetMathLibrary.MakeVector` 0.0 0.0 (`self.VerticalOffsetHB`)) false false)
  (set `self.VerticalWorldOffsetHB` (- _returnvalue_z _returnvalue_z_2))
  ;;[0.4098 0.3255 0.8314] Set Scale Hovering Button Timeline Speed
  (`TimelineComponent.SetPlayRate` (`self.HoveringButtonScaleTimeline`) (/ 1.0 (`self.ScalingSpeedHB`)))
  ;;[0.7133 0.3255 0.8314] Set Down Scale Hovering Button Timeline Speed
  (`TimelineComponent.SetPlayRate` (`self.HoveringButtonDownScaleTimeline`) (/ 1.0 (/ (`self.ScalingSpeedHB`) 1.25)))
  ;;[0.3255 0.5216 0.8314] Set Hovering Button Timeline Speed
  (`TimelineComponent.SetPlayRate` (`self.HoverButtonTimeline`) (/ 1.0 (`self.HoveringSpeedHB`))))