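; BP_CrackedNutEnemy is an enemy that is launched out of a nut.
; SpawnFromNut pushes its character movement along a given direction scaled by SpawnForce and enables actor collision.
; TakesDamages spawns a BP_DeadEnnemi at its transform, calls Planted on the score component, then destroys the actor.
; The construction script sets its Name enum, and BeginPlay defers to the parent class.
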(event `self.ReceiveBeginPlay`
  (`parent.ReceiveBeginPlay`))

(event `SpawnFromNut`
  (params (ForceDirection :type "Vector Structure"))
  (`CharacterMovementComponent.AddForce` (`self.CharacterMovement`) (* ForceDirection (`self.SpawnForce`)))
  (`self.SetActorEnableCollision` true))

(fn `TakesDamages`
  (`|SpawnActorFromClass` "/Game/Gameplay/Enemies/BP_DeadEnnemi.BP_DeadEnnemi_C" (`self.GetTransform`) "Undefined" "OverrideRootScale" null null null)
  (`/Game/Gameplay/Enemies/EnemiesBlueprints/BP_ScoreComponent.Planted` (`self.BP_ScoreComponent`))
  (`self.K2_DestroyActor`))

(fn `UserConstructionScript`
  (`parent.UserConstructionScript`)
  (set `self.Name` "NewEnumerator1"))