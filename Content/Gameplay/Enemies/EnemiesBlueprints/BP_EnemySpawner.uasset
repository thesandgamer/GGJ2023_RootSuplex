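; Enemy wave spawner that spawns carrot, nut and artichoke enemies in timed waves defined by DT_EnemyWave.
; Each wave reads the row named after WaveCount, increments that counter and schedules the next wave from the row's timer, stopping when no row is found.
; Spawn points come from line traces starting high at random X around the actor and Y around world zero.
; Each hit spawns an enemy and fires EnemyCreated.
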(event `self.ReceiveBeginPlay`
  (bind _returnvalue (`|GetDataTableRow` "/Game/Gameplay/Enemies/DT_EnemyWave.DT_EnemyWave" (`KismetStringLibrary.Conv_StringToName` (`KismetStringLibrary.Conv_IntToString` (`self.WaveCount`))))
    (:`then`
      (bind (_carrotcount _nutcount _artichokecount _wavetimer) (break `/Game/Gameplay/Enemies/SEnemyWaveStruct` _returnvalue))
      (`self.SpawnEnemies` _carrotcount _nutcount _artichokecount)
      (`KismetSystemLibrary.K2_SetTimerDelegate` (delegate `Next Wave`) (`KismetMathLibrary.Conv_IntToDouble` _wavetimer)))))

(event `Next Wave`
  (bind _returnvalue (`|GetDataTableRow` "/Game/Gameplay/Enemies/DT_EnemyWave.DT_EnemyWave" (`KismetStringLibrary.Conv_StringToName` (`KismetStringLibrary.Conv_IntToString` (`self.WaveCount`))))
    (:`then`
      (bind (_carrotcount _nutcount _artichokecount _wavetimer) (break `/Game/Gameplay/Enemies/SEnemyWaveStruct` _returnvalue))
      (`KismetSystemLibrary.PrintString` (`KismetStringLibrary.Conv_IntToString` _carrotcount))
      (`self.SpawnEnemies` _carrotcount _nutcount _artichokecount)
      (`KismetSystemLibrary.K2_SetTimerDelegate` (delegate `Next Wave`) (`KismetMathLibrary.Conv_IntToDouble` _wavetimer)))))

(fn `RandomSpawnLocationGenerator`
  (returns (ReturnValue :type Boolean) (`Out Hit Location` :type "Vector Structure"))
  (locals (RayVector :type "Vector Structure") (RayLong :type "Float (double-precision)" :default 200000.0))
  (bind _maxspawnx (`self.MaxSpawnX`))
  (bind _maxspawny (`self.MaxSpawnY`))
  (bind _returnvalue (+ 0.0 (`KismetMathLibrary.RandomFloatInRange` (* _maxspawny -1.0) _maxspawny)))
  (bind _returnvalue_2 (+ (.x (.location (`self.GetTransform`))) (`KismetMathLibrary.RandomFloatInRange` (* _maxspawnx -1.0) _maxspawnx)))
  (set `local.RayVector` (`KismetMathLibrary.MakeVector` _returnvalue_2 _returnvalue 2000.0))
  (bind (_outhit _returnvalue_3) (`KismetSystemLibrary.LineTraceSingle` :`Start` (`KismetMathLibrary.MakeVector` _returnvalue_2 _returnvalue 20000.0) :`End` (* (`KismetMathLibrary.Vector_Down`) (`local.RayLong`)) :`TraceChannel` "TraceTypeQuery1" :`bTraceComplex` true :`DrawDebugType` "ForDuration"))
  (if _returnvalue_3
    (return _returnvalue_3 (`.ImpactPoint` (`GameplayStatics.BreakHitResult` _outhit)))
    (else
      (return false (0.0 0.0 0.0)))))

(fn `SpawnEnemies`
  (params (CarrotCount :type Integer) (NoisetteCount :type Integer) (ArtichautCount :type Integer))
  (set `self.WaveCount` (+ (`self.WaveCount`) 1))
  (`|ExecutionSequence`
    (:`then_0`
      (for _ (range 1 (+ CarrotCount 1))
        (bind (_returnvalue _out_hit_location) (`self.RandomSpawnLocationGenerator`))
        (if _returnvalue
          (bind _returnvalue_2 (`|SpawnActorFromClass` "/Game/Gameplay/Enemies/EnemiesBlueprints/BP_CarrotEnemy.BP_CarrotEnemy_C" (`KismetMathLibrary.MakeTransform` _out_hit_location) "AdjustIfPossibleButAlwaysSpawn" "OverrideRootScale" null null))
          (`self.EnemyCreated` _returnvalue_2))))
    (:`then_1`
      (for _ (range 1 (+ NoisetteCount 1))
        (bind (_returnvalue_3 _out_hit_location_2) (`self.RandomSpawnLocationGenerator`))
        (if _returnvalue_3
          (bind _returnvalue_4 (`|SpawnActorFromClass` "/Game/Gameplay/Enemies/EnemiesBlueprints/BP_NutEnemy.BP_NutEnemy_C" (`KismetMathLibrary.MakeTransform` _out_hit_location_2) "AdjustIfPossibleButAlwaysSpawn" "OverrideRootScale" null null))
          (`self.EnemyCreated` _returnvalue_4))))
    (:`then_2`
      (for _ (range 1 (+ ArtichautCount 1))
        (bind (_returnvalue_5 _out_hit_location_3) (`self.RandomSpawnLocationGenerator`))
        (if _returnvalue_5
          (bind _returnvalue_6 (`|SpawnActorFromClass` "/Game/Gameplay/Enemies/EnemiesBlueprints/BP_ArtichokeEnemy.BP_ArtichokeEnemy_C" (`KismetMathLibrary.MakeTransform` _out_hit_location_3) "AdjustIfPossibleButAlwaysSpawn" "OverrideRootScale" null null))
          (`self.EnemyCreated` _returnvalue_6))))))

(fn `UserConstructionScript`)