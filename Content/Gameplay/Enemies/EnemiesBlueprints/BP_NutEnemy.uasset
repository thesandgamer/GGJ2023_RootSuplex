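; BP_NutEnemy is a nut enemy that cracks when damaged near a stone zone or another nut enemy.
; TakesDamages runs a small sphere trace at the actor's location and looks for hits of exactly those two classes.
; On a match it spawns BP_CrackedNutEnemy in place, keeping only yaw, and destroys itself; otherwise nothing happens.
; The event graph is empty, and the trace leaves debug drawing on.
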(fn `TakesDamages`
  (bind (_returnvalue_roll _returnvalue_pitch _returnvalue_yaw) (`KismetMathLibrary.BreakRotator` (`self.K2_GetActorRotation`)))
  (bind _returnvalue (`self.K2_GetActorLocation`))
  (bind (_outhits _returnvalue_2) (`KismetSystemLibrary.SphereTraceMultiByProfile` :`Start` _returnvalue :`End` _returnvalue :`Radius` 150.0 :`DrawDebugType` "ForDuration"))
  (if _returnvalue_2
    (for _array_element _outhits
      (bind _returnvalue_3 (`GameplayStatics.GetObjectClass` (`.HitActor` (`GameplayStatics.BreakHitResult` _array_element))))
      (if (or (== _returnvalue_3 "/Game/Gameplay/Enemies/BP_StoneZone.BP_StoneZone_C") (== _returnvalue_3 "BP_NutEnemy_C"))
        (`|SpawnActorFromClass` "/Game/Gameplay/Enemies/EnemiesBlueprints/BP_CrackedNutEnemy.BP_CrackedNutEnemy_C" (`KismetMathLibrary.MakeTransform` (`self.K2_GetActorLocation`) (`KismetMathLibrary.MakeRotator` 0.0 0.0 _returnvalue_yaw)) "Undefined" "OverrideRootScale" null null)
        (`self.K2_DestroyActor`)
        (return)))))

(fn `UserConstructionScript`
  (`parent.UserConstructionScript`))