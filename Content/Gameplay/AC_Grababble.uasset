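; Actor component that makes its owning actor something the third-person character can pick up, drop or plant.
; Grabbing checks CanBeGrabbed, passes the character's GrabPoint to Grab and returns whether the grab was allowed.
; Grab snaps the owner to that point and disables its collision, while Drop detaches it in world space and restores collision.
; Plant simply destroys the owner.
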(fn `Drop`
  (`Actor.K2_DetachFromActor` (`self.GetOwner`) "KeepWorld" "KeepWorld" "KeepRelative")
  (`Actor.SetActorEnableCollision` (`self.GetOwner`) true))

(fn `Grab`
  (params (Parent :type "SceneComponent Object Reference"))
  (`Actor.K2_AttachToComponent` (`self.GetOwner`) Parent "None" "SnapToTarget" "SnapToTarget" "KeepRelative" true)
  (`Actor.SetActorEnableCollision` (`self.GetOwner`) false))

(fn `Grabbing`
  (params (WhoGrabbed :type "Actor Object Reference"))
  (returns (CanBeGrabbed :type Boolean))
  (bind _canbegrabbed (`self.CanBeGrabbed`))
  (if _canbegrabbed
    (`self.Grab` (`/Game/Gameplay/BP_ThirdPersonCharacter.GrabPoint` (cast `/Game/Gameplay/BP_ThirdPersonCharacter` WhoGrabbed :!pure true))))
  (return _canbegrabbed))

(fn `Plant`
  (`Actor.K2_DestroyActor` (`self.GetOwner`)))