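; Countdown timer Blueprint that shows the remaining minutes and seconds in a W_Timer widget.
; On BeginPlay it reuses existing timer widgets or creates one, sets the time from CountdownMax, and starts counting after a short delay.
; A looping one-second timer decrements the time and refreshes the widget, with start and finish dispatchers broadcast.
; Events also allow pausing, resuming and resetting to zero, which happens automatically on finish.
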(event `CreateTimer`
  (bind _foundwidgets (`WidgetBlueprintLibrary.GetAllWidgetsOfClass` "/Game/Gameplay/Timer/W_Timer.W_Timer_C" false))
  (if (`KismetArrayLibrary.Array_IsNotEmpty` _foundwidgets)
    (for _array_element _foundwidgets
      (set `self.TimerWidget` _array_element)
      (`self.SetupTimer` :!label _label))
    (else
      (bind _returnvalue (`|CreateWidget` "/Game/Gameplay/Timer/W_Timer.W_Timer_C"))
      (bind _output_get (set `self.TimerWidget` _returnvalue))
      (`UserWidget.AddToViewport` _output_get 0)
      (goto _label))))

(event `self.ReceiveBeginPlay`
  (`self.CreateTimer`)
  (`KismetSystemLibrary.Delay` 2.0)
  (`self.StartTimer`))

(event `PauseTimer`
  ;[1 1 1] Comment
  (`KismetSystemLibrary.K2_PauseTimerHandle` (`self.Timer`)))

(event `StartTimer`
  (`self.SetWidgetTimer`)
  (bind _returnvalue (`KismetSystemLibrary.K2_SetTimerDelegate` (delegate `TimePass`) 1.0 true))
  (set `self.Timer` _returnvalue)
  (`self.Ev_TimerStarted`))

(event `PlayTimer`
  ;[1 1 1] Comment
  (`KismetSystemLibrary.K2_UnPauseTimerHandle` (`self.Timer`)))

(event `ResetTimer`
  ;[1 1 1] Comment
  (set `self.CurrentTime` 0.0)
  (`KismetSystemLibrary.K2_ClearAndInvalidateTimerHandle` (`self.Timer`)))

(event `TimePass`
  (bind _currenttime (`self.CurrentTime`))
  (`/Engine/EditorBlueprintResources/StandardMacros.DecrementFloat` _currenttime
    (:`  `
      (`self.SetWidgetTimer`)
      (if (<= _currenttime 0.0)
        (`self.TimerFinished`)))))

(event `TimerFinished`
  (`self.Ev_TimerFinished`)
  (`self.ResetTimer`))

(fn `SetupTimer`
  (bind (_countdownmax_min _countdownmax_sec) (break `/Game/Gameplay/Timer/Str_Time` (`self.CountdownMax`)))
  (set `self.CurrentTime` (`KismetMathLibrary.Conv_IntToDouble` (+ (* _countdownmax_min 60) _countdownmax_sec)))
  (`self.SetWidgetTimer`))

(fn `SetWidgetTimer`
  (bind _timerwidget (`self.TimerWidget`))
  (bind _returnvalue (`KismetMathLibrary.FromSeconds` (`self.CurrentTime`)))
  (`/Game/Gameplay/Timer/W_Timer.SetSec` _timerwidget (`KismetMathLibrary.GetSeconds` _returnvalue))
  (`/Game/Gameplay/Timer/W_Timer.SetMin` _timerwidget (`KismetMathLibrary.GetMinutes` _returnvalue))
  (return))

(fn `UserConstructionScript`)