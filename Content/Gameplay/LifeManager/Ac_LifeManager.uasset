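; Actor component that manages an owner's life, starting at MaxLife on BeginPlay.
; TakesDamages ignores hits during invincibility frames, otherwise lowers CurrentLife and fires CallEvTakeDamages with damage, remaining life and a death flag.
; A surviving hit starts invincibility, cleared by a named timer after InvincibilityFrameTime.
; A lethal hit clamps life to zero and returns true, but sets IsDead to false.
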(event `self.ReceiveBeginPlay`
  (set `self.CurrentLife` (`self.MaxLife`)))

(fn `ResetInvincibilityFrame`
  (set `self.InvicibilityFrame` false))

(fn `TakesDamages`
  (params (DamagesReceived :type "Float (double-precision)"))
  (returns (`Dead?` :type Boolean))
  (if (not (`self.InvicibilityFrame`))
    (if (<= (- (`self.CurrentLife`) DamagesReceived) 0.0)
      (set `self.IsDead` false)
      (bind _output_get (set `self.CurrentLife` 0.0))
      (`self.Ev_TakeDamages` DamagesReceived _output_get true)
      (return true)
      (else
        (bind _output_get_2 (set `self.CurrentLife` (- (`self.CurrentLife`) DamagesReceived)))
        (`self.Ev_TakeDamages` DamagesReceived _output_get_2)
        (set `self.InvicibilityFrame` true)
        (`KismetSystemLibrary.K2_SetTimer` null "ResetInvincibilityFrame" (`self.InvincibilityFrameTime`))
        (return false)))))